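; Interactable door prop that swings open and closed on alternate interactions.
; OnInteraction drives a FlipFlop that plays or reverses a timeline and calls Door() on each toggle.
; The timeline lerps the relative rotation of SMDoor up to a 90-degree turn.
; The construction script applies custom meshes to the door and a second static mesh component, so the prop's look can vary.
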(event Custom|OnInteraction
  (Utilities|FlowControl|FlipFlop
    (:A
      (Utilities|FlowControl|Sequence
        (:then_0
          (CallFunction|Door))
        (:then_1
          (bind _newtrack_0 (Timeline|Timeline_0 Play)
            (:Update
              (Transformation|SetRelativeRotation (Variables|Default|GetSM_Door) (Math|Rotator|Lerp(Rotator) "0, 0, 0" "0,90.000000, 0" _newtrack_0) false false))))))
    (:B
      (Utilities|FlowControl|Sequence
        (:then_0
          (Timeline|Timeline_0 Reverse))
        (:then_1
          (CallFunction|Door))))))

(fn ConstructionScript
  (Components|StaticMesh|SetStaticMesh (Variables|Default|GetStaticMesh) (Variables|Default|GetCustomStaticMesh_1))
  (Components|StaticMesh|SetStaticMesh (Variables|Default|GetSM_Door) (Variables|Default|GetCustomStaticMesh_0)))