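; Interactable chest prop whose second mesh swings open on proximity and which shows a widget when interacted with.
; Tick compares distance to Radius, playing or reversing a timeline that rotates the mesh and toggling a text render using the Visible flag.
; OnInteraction adds the widget to the viewport after a short delay, sets Visible, and calls Chest.
; The construction script applies custom meshes to both chest parts.
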(event Custom|OnInteraction
  (Utilities|FlowControl|Sequence
    (:then_1
      (Utilities|FlowControl|Delay 0.2)
      (bind _returnvalue (UserInterface|CreateWidget 0))
      (UserInterface|Viewport|AddtoViewport _returnvalue 0))
    (:then_2
      (Variables|Default|SetVisible true))
    (:then_3
      (CallFunction|Chest))))

(event EventTick
  (params (DeltaSeconds :type Float%20%28single-precision%29))
  (bind _visible (Variables|Default|GetVisible))
  (bind _textrender (Variables|Default|GetTextRender))
  (if (< (Transformation|GetDistanceTo (Components|GetOwner (Variables|Default|GetStaticMesh)) 0) (Variables|Default|GetRadius))
    (Rendering|SetVisibility _textrender (not _visible) false)
    (bind _rotator_chest_1 (Timeline|Timeline_0 Play)
      (:Update
        (Transformation|SetRelativeRotation (Variables|Default|GetStaticMesh1) (Math|Rotator|Lerp(Rotator) "0,0.000000,0.000000" "0, 0,60.000000" _rotator_chest_1) false false)))
    (else
      (Rendering|SetVisibility _textrender _visible false)
      (Timeline|Timeline_0 Reverse))))

(fn ConstructionScript
  (Components|StaticMesh|SetStaticMesh (Variables|Default|GetStaticMesh) (Variables|Default|GetCustomStaticMesh_1))
  (Components|StaticMesh|SetStaticMesh (Variables|Default|GetStaticMesh1) (Variables|Default|GetCustomStaticMesh_2)))